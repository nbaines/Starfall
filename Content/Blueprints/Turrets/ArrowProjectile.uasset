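; Arrow projectile, filed under turrets, that knocks back the first-person character on impact and then fades away.
; On hit, it applies a velocity-scaled impulse to that character's movement, while any other hit waits briefly before fading.
; A FadeOut timeline scales the Niagara effect and drives the arrow material's opacity from the squared Z curve, then destroys the actor.
; Physics-impulse and emissive-fade nodes are left unconnected.
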(event EventBeginPlay)

(event Collision|EventActorBeginOverlap
  (params (OtherActor :type Actor%20Object%20Reference)))

(event EventTick
  (params (DeltaSeconds :type Float%20%28single-precision%29)))

(event Collision|EventHit
  (params (MyComp :type Primitive%20Component%20Object%20Reference) (Other :type Actor%20Object%20Reference) (OtherComp :type Primitive%20Component%20Object%20Reference) (bSelfMoved :type Boolean) (HitLocation :type Vector :default "0, 0, 0") (HitNormal :type Vector :default "0, 0, 0") (NormalImpulse :type Vector :default "0, 0, 0") (Hit :type Hit%20Result%20Structure%20%28by%20ref%29))
  (bind _asfirst_person_character (Utilities|Casting|CastToFirstPersonCharacter Other)
    (:then
      (Physics|AddImpulse (Variables|/Script/Engine.Character|GetCharacterMovement _asfirst_person_character) (* (Transformation|GetVelocity) 5e+01) false)
      (bind (_direction _xscale _yscale _zscale) (Timeline|Fade%20Out Play)
        (:Update
          (Transformation|SetWorldScale3D (Variables|Default|GetNiagara) (Math|Vector|MakeVector _xscale _yscale _zscale))
          (Rendering|Material|SetScalarParameterValueonMaterials (Variables|Default|Getsm_arrow) "Opacity" (Math|Float|Square _zscale)))
        (:Finished
          (Actor|DestroyActor))))
    (:CastFailed
      (Utilities|FlowControl|Delay 1.0)
      (Timeline|Fade%20Out Play))))

(fn ConstructionScript)