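; Arrow turret that sweeps between yaw limits around its starting rotation and attacks the player on sight.
; Tick drives the idle sweep with pauses at each end, plus a timeline that levels the turret after an alert.
; PawnSensing triggers alert visuals, limit-checked RInterpTo tracking and cooldown-gated arrows launched by impulse toward the player.
; A timer set after each shot's cooldown clears PlayerSpotted, returning it to idle.
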(event OnSeePawn(PawnSensing)
  (params (Pawn :type Pawn%20Object%20Reference))
  (bind _returnvalue (Transformation|GetActorRotation))
  (bind _returnvalue_2 (Transformation|GetActorLocation))
  (bind _asfirst_person_character (Utilities|Casting|CastToFirstPersonCharacter Pawn))
  (Variables|Default|SetplayerSpotted true)
  ;[0.2244 0.5594 0.9167] Rotate turret to face player
  (Utilities|FlowControl|Sequence
    (:then_0
      (CallFunction|EnableAlert)
      (bind _newtrack_0 (Timeline|Timeline_0 PlayFromStart)
        (:Update
          (if (not (>= (.yaw (Math|Interpolation|RInterpTo (Transformation|GetActorRotation) (Math|Rotator|FindLookatRotation _returnvalue_2 (Transformation|GetActorLocation _asfirst_person_character)) _newtrack_0 5.0)) (Variables|Default|GetrightRotationLim)))
            (if (not (<= (.yaw (Math|Interpolation|RInterpTo (Transformation|GetActorRotation) (Math|Rotator|FindLookatRotation _returnvalue_2 (Transformation|GetActorLocation _asfirst_person_character)) _newtrack_0 5.0)) (Variables|Default|GetleftRotationLim)))
              (Transformation|SetActorRotation (Math|Rotator|MakeRotator (.roll (Math|Interpolation|RInterpTo (Transformation|GetActorRotation) (Math|Rotator|FindLookatRotation _returnvalue_2 (Transformation|GetActorLocation _asfirst_person_character)) _newtrack_0 5.0)) (.pitch (Math|Interpolation|RInterpTo (Transformation|GetActorRotation) (Math|Rotator|FindLookatRotation _returnvalue_2 (Transformation|GetActorLocation _asfirst_person_character)) _newtrack_0 5.0)) (.yaw (Math|Interpolation|RInterpTo (Transformation|GetActorRotation) (Math|Rotator|FindLookatRotation _returnvalue_2 (Transformation|GetActorLocation _asfirst_person_character)) _newtrack_0 5.0))))
              (Utilities|FlowControl|DoOnce false) ; enters at Reset
            )))))
    (:then_1
      ;[0.8802 0.4162 0.1238 0.765] Shoot arrow
      (if (Variables|Default|GetcanShoot)
        (bind _returnvalue_3 (Game|SpawnActorfromClass "/Game/Blueprints/Turrets/ArrowProjectile.ArrowProjectile_C" (Transformation|GetWorldTransform (Variables|Default|GetArrowSpawnpoint)) "Undefined" 0 0))
        (Physics|AddImpulse (Variables|/Game/Blueprints/Turrets/ArrowProjectile.ArrowProjectile_C|Getsm_arrow _returnvalue_3) (* (Math|Vector|GetUnitDirection(Vector) _returnvalue_2 (Transformation|GetActorLocation _asfirst_person_character)) 2e+03) "None" true)
        (Variables|Default|SetcanShoot false)
        (Utilities|FlowControl|Delay (Variables|Default|GetFireCooldown)) ; Cooldown btwn shots
        (Variables|Default|SetcanShoot true)
        (Utilities|Time|SetTimerbyFunctionName 0 "resetPlayerSpotted" (Variables|Default|GetAlertCooldown)) ; Exit "alert" state if haven't seen player after 'x' sec\n(i.e. return to idle rotation)
      ))))

(event EventBeginPlay
  (Variables|Default|SetInitialWorldRotation (Transformation|GetActorRotation))
  (Variables|Default|SetleftRotationLim (+ (.yaw (Variables|Default|GetInitialWorldRotation)) (/ (Variables|Default|GetMaxRotationDeg) -2.0)))
  (Variables|Default|SetrightRotationLim (+ (.yaw (Variables|Default|GetInitialWorldRotation)) (/ (Variables|Default|GetMaxRotationDeg) 2.0))))

(event Collision|EventActorBeginOverlap
  (params (OtherActor :type Actor%20Object%20Reference)))

(event EventTick
  (params (DeltaSeconds :type Float%20%28single-precision%29))
  (bind _returnvalue (Transformation|GetActorRotation))
  (bind _rightrotationlim (Variables|Default|GetrightRotationLim))
  (bind _leftrotationlim (Variables|Default|GetleftRotationLim))
  ;[0.7969 0.7688 0.2117 0.593] Idle: continously rotate turret
  (if (not (Variables|Default|GetplayerSpotted))
    (Transformation|AddActorLocalRotation (Math|Rotator|MakeRotator 0.0 0.0 (* DeltaSeconds (Variables|Default|GetIdleRotSpeed))) false false)
    (Utilities|FlowControl|Sequence
      (:then_0
        (Utilities|FlowControl|DoOnce false
          (:Completed
            (CallFunction|DisableAlert)
            ;[0.5738 0.1441 0.8385 0.718] Reset turret rotation
            (bind _newtrack_0 (Timeline|Timeline_1 PlayFromStart)
              (:Update
                (Transformation|SetActorRotation (Math|Rotator|Lerp(Rotator) (Math|Rotator|MakeRotator (.roll _returnvalue) (.pitch _returnvalue) (.yaw _returnvalue)) (Math|Rotator|MakeRotator 0.0 0.0 (.yaw _returnvalue)) _newtrack_0)))))))
      (:then_1
        (if (Variables|Default|GetidleRotRight)
          ;[0.1747 1 0.9403 0.671] Right rotation
          (if (>= _rightrotationlim 1.8e+02)
            (if (== (+ -1.8e+02 (- (Variables|Default|GetrightRotationLim) 1.8e+02)) 0.0)
              (Variables|Default|SetIdleRotSpeed 0.0)
              (Utilities|FlowControl|Delay 2.0)
              (Variables|Default|SetIdleRotSpeed -4e+01)
              (Variables|Default|SetidleRotRight false))
            (elif (>= (.yaw (Transformation|GetActorRotation)) (- _rightrotationlim 0.5))
              (Variables|Default|SetIdleRotSpeed 0.0)
              (Utilities|FlowControl|Delay 2.0)
              (Variables|Default|SetIdleRotSpeed -4e+01)
              (Variables|Default|SetidleRotRight false)))
          (else
            ;[1 0.1747 0.6836 0.671] Left rotation
            (if (<= _leftrotationlim -1.8e+02)
              (if (== (+ 1.8e+02 (- (Variables|Default|GetleftRotationLim) -1.8e+02)) 0.0)
                (Variables|Default|SetIdleRotSpeed 0.0)
                (Utilities|FlowControl|Delay 2.0)
                (Variables|Default|SetIdleRotSpeed 4e+01)
                (Variables|Default|SetidleRotRight true))
              (elif (<= (.yaw (Transformation|GetActorRotation)) (+ _leftrotationlim 0.5))
                (Variables|Default|SetIdleRotSpeed 0.0)
                (Utilities|FlowControl|Delay 2.0)
                (Variables|Default|SetIdleRotSpeed 4e+01)
                (Variables|Default|SetidleRotRight true)))))))))

(fn ConstructionScript)

(fn ResetPlayerSpotted
  (Variables|Default|SetplayerSpotted false)
  (return))

(fn EnableAlert
  (Rendering|SetVisibility (Variables|Default|GetBP_MagicCircle_Idle) false false)
  (Rendering|SetVisibility (Variables|Default|GetBP_MagicCircle_Alert) true false)
  (Rendering|Material|SetMaterial (Variables|Default|Getsm_turret) 1 "/Game/Developers/Sarah/Collections/Turrets/Turret01/lambert10SG1.lambert10SG1") ; Eye background
  (Rendering|Material|SetMaterial (Variables|Default|Getsm_turret) 3 "/Game/Developers/Sarah/Collections/Turrets/Turret02/purplerender02_Mat.purplerender02_Mat") ; Eye gem
  (Rendering|Material|SetMaterial (Variables|Default|Getsm_turret) 0 "/Game/Developers/Sarah/Collections/Turrets/Turret02/purplerender02_Mat.purplerender02_Mat") ; Rear gem
  (return))

(fn DisableAlert
  (Rendering|SetVisibility (Variables|Default|GetBP_MagicCircle_Idle) true false)
  (Rendering|SetVisibility (Variables|Default|GetBP_MagicCircle_Alert) false false)
  (Rendering|Material|SetMaterial (Variables|Default|Getsm_turret) 1 "/Game/Developers/Sarah/Collections/Turrets/Turret02/lambert4SG1.lambert4SG1") ; Eye background
  (Rendering|Material|SetMaterial (Variables|Default|Getsm_turret) 3 "/Game/Developers/Sarah/Collections/Turrets/Turret02/phongE1SG1.phongE1SG1") ; Eye gem
  (Rendering|Material|SetMaterial (Variables|Default|Getsm_turret) 0 "/Game/Developers/Sarah/Collections/Turrets/Turret02/phongE1SG1.phongE1SG1") ; Rear gem
  (return))