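; EndStar_BP is a collectible star pickup that the player gathers in a level.
; When a FirstPersonCharacter overlaps Sphere1, it calls CollectedRequiredStar on the character, records the current level name with the GameManager game instance via SetStarCollector, then destroys itself.
; Tick slowly spins the Sphere component around its yaw axis.
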(event OnComponentBeginOverlap(Sphere1)
  (params (OverlappedComponent :type Primitive%20Component%20Object%20Reference) (OtherActor :type Actor%20Object%20Reference) (OtherComp :type Primitive%20Component%20Object%20Reference) (OtherBodyIndex :type Integer) (bFromSweep :type Boolean) (SweepResult :type Hit%20Result%20Structure%20%28by%20ref%29))
  (bind _asfirst_person_character (Utilities|Casting|CastToFirstPersonCharacter OtherActor))
  (Default|CollectedRequiredStar _asfirst_person_character)
  (bind _asgame_manager (Utilities|Casting|CastToGameManager (Game|GetGameInstance)))
  (bind _returnvalue (Game|GetCurrentLevelName true))
  (Default|SetStarCollector _asgame_manager _returnvalue)
  (Actor|DestroyActor))

(event EventBeginPlay)

(event Collision|EventActorBeginOverlap
  (params (OtherActor :type Actor%20Object%20Reference)))

(event EventTick
  (params (DeltaSeconds :type Float%20%28single-precision%29))
  (Transformation|AddRelativeRotation (Variables|Default|GetSphere) (Math|Rotator|MakeRotator 0.0 0.0 (* DeltaSeconds 4e+01)) false false))

(fn ConstructionScript)